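; Shop door Blueprint that opens a final-decision UI widget (WB_2DFinalDecision) when interacted with.
; The first Interact creates and caches the widget with a reference to this door, sets its image, adds it to the viewport and shows the mouse cursor.
; Later interactions reuse the cached widget through a DoOnce that refreshes the image and re-adds it, with Resetwidget re-arming that gate.
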(event Custom|Reset%20widget
  (Utilities|FlowControl|DoOnce false) ; enters at Reset
)

(event EventInteract
  (Utilities|IsValid (Variables|Default|GetWidgetRef)
    (:Is%20Valid
      (Utilities|FlowControl|DoOnce false
        (:Completed
          (Class|Image|SetBrush (Variables|/Game/Doors/2D/WB_2DFinalDecision.WB_2DFinalDecision_C|GetImage_0 (Variables|Default|GetWidgetRef)) (Utilities|Struct|MakeSlateBrush "Image" "NoTile" "NoMirror" "(X=32.000000,Y=32.000000)" "(Left=0.000000,Top=0.000000,Right=0.000000,Bottom=0.000000)" "(SpecifiedColor=(R=1.000000,G=1.000000,B=1.000000,A=1.000000),ColorUseRule=UseColor_Specified)" "(CornerRadii=(X=0.000000,Y=0.000000,Z=0.000000,W=1.000000),Color=(SpecifiedColor=(R=0.000000,G=0.000000,B=0.000000,A=0.000000),ColorUseRule=UseColor_Specified),Width=0.000000,RoundingType=HalfHeightRadius,bUseBrushTransparency=False)" (Variables|Default|GetIn%20Brush%20Image)))
          (UserInterface|Viewport|AddtoViewport (Variables|Default|GetWidgetRef) 0))))
    (:Is%20Not%20Valid
      (bind _returnvalue (UserInterface|CreateWidget "/Game/Doors/2D/WB_2DFinalDecision.WB_2DFinalDecision_C" 0 self))
      (bind _output_get (Variables|Default|SetWidgetRef _returnvalue))
      (Class|Image|SetBrush (Variables|/Game/Doors/2D/WB_2DFinalDecision.WB_2DFinalDecision_C|GetImage_0 _output_get) (Utilities|Struct|MakeSlateBrush "Image" "NoTile" "NoMirror" "(X=32.000000,Y=32.000000)" "(Left=0.000000,Top=0.000000,Right=0.000000,Bottom=0.000000)" "(SpecifiedColor=(R=1.000000,G=1.000000,B=1.000000,A=1.000000),ColorUseRule=UseColor_Specified)" "(CornerRadii=(X=0.000000,Y=0.000000,Z=0.000000,W=1.000000),Color=(SpecifiedColor=(R=0.000000,G=0.000000,B=0.000000,A=0.000000),ColorUseRule=UseColor_Specified),Width=0.000000,RoundingType=HalfHeightRadius,bUseBrushTransparency=False)" (Variables|Default|GetIn%20Brush%20Image)))
      (UserInterface|Viewport|AddtoViewport _returnvalue 0)
      (Variables|/Script/Engine.PlayerController|SetbShowMouseCursor (Game|GetPlayerController 0) true))))

(fn ConstructionScript)