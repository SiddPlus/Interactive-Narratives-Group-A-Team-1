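; Door trigger Blueprint that opens the WB_2DFinalDecision menu on interaction.
; The first Interact creates the widget with itself as the Door reference, caches it, adds it to the viewport and shows the mouse cursor.
; Later interactions re-add the cached widget through a DoOnce gate, which the Resetwidget event re-arms.
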(event Custom|Reset%20widget
  (Utilities|FlowControl|DoOnce false) ; enters at Reset
)

(event EventInteract
  (Utilities|IsValid (Variables|Default|GetWB%202DMenu)
    (:Is%20Valid
      (Utilities|FlowControl|DoOnce false
        (:Completed
          (UserInterface|Viewport|AddtoViewport (Variables|Default|GetWB%202DMenu) 0))))
    (:Is%20Not%20Valid
      (bind _returnvalue (UserInterface|CreateWidget "/Game/Doors/2D/WB_2DFinalDecision.WB_2DFinalDecision_C" 0 self))
      (Variables|Default|SetWB%202DMenu _returnvalue)
      (UserInterface|Viewport|AddtoViewport _returnvalue 0)
      (Variables|/Script/Engine.PlayerController|SetbShowMouseCursor (Game|GetPlayerController 0) true))))

(fn ConstructionScript)